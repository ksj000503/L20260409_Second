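; BP_Rocket is a projectile that homes in on the first BP_Target actor found in the level at BeginPlay.
; Overlapping any actor spawns a Niagara explosion and 2D sound, applies damage credited to the first player controller, and destroys the rocket.
; A short lifespan limits its flight, with an equal Delay meant to spawn the explosion effect as it expires, without sound or damage.
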(event `self.ReceiveBeginPlay`
  (bind _outactors (`GameplayStatics.GetAllActorsOfClass` "/Game/Blueprint/BP_Target.BP_Target_C"))
  (set `ProjectileMovementComponent.HomingTargetComponent` (`Actor.RootComponent` (`|GetArrayItem` _outactors)) (`self.ProjectileMovement`))
  (`self.SetLifeSpan` 3.0)
  (`KismetSystemLibrary.Delay` 3.0)
  (`NiagaraFunctionLibrary.SpawnSystemAtLocation` "/Game/NiagaraExamples/FX_Explosions/NS_Explosion_Medium.NS_Explosion_Medium" (`self.K2_GetActorLocation`)))

(event `self.ReceiveActorBeginOverlap`
  (params (OtherActor :type "Actor Object Reference"))
  (`NiagaraFunctionLibrary.SpawnSystemAtLocation` "/Game/NiagaraExamples/FX_Explosions/NS_Explosion_Medium.NS_Explosion_Medium" (`self.K2_GetActorLocation`))
  (`GameplayStatics.SpawnSound2D` "/Game/Sounds/MS_Explosion.MS_Explosion" 1.0 1.0 0.0 null)
  (`GameplayStatics.ApplyDamage` OtherActor 10.0 (`GameplayStatics.GetPlayerController` 0) self)
  (`self.K2_DestroyActor`))

(fn `UserConstructionScript`)