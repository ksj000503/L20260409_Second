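; Player-controlled flying pawn that constantly moves forward and fires rockets.
; Tick feeds the forward vector into movement input, while the RightLeft and UpDown axes apply local roll and pitch scaled by RotatorSpeed and delta time.
; The Fire input calls Fire, which spawns BP_Rocket alternately from two Arrow components by flipping the IsOneTwo flag, with the pawn as owner and instigator.
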(event `self.ReceiveBeginPlay`)

(event `self.ReceiveTick`
  (params (DeltaSeconds :type "Float (single-precision)"))
  ; 전진
  (`self.AddMovementInput` (`self.GetActorForwardVector`)))

(event `InputAction|Fire`
  (params (Key :type "Key Structure"))
  ; 미사일 발사
  (:`Pressed`
    (`self.Fire`)))

(event `InputAxis|RightLeft`
  (params (AxisValue :type "Float (single-precision)"))
  ; Roll 회전
  (`self.K2_AddActorLocalRotation` (`KismetMathLibrary.MakeRotator` (* AxisValue (`self.RotatorSpeed`) (`GameplayStatics.GetWorldDeltaSeconds`)))))

(event `InputAxis|UpDown`
  (params (AxisValue :type "Float (single-precision)"))
  ; Pitch 회전
  (`self.K2_AddActorLocalRotation` (`KismetMathLibrary.MakeRotator` 0.0 (* AxisValue (`self.RotatorSpeed`) (`GameplayStatics.GetWorldDeltaSeconds`)))))

(fn `Fire`
  (if (`self.bIsOneTwo`)
    (`|SpawnActorFromClass` "/Game/Blueprint/BP_Rocket.BP_Rocket_C" (`SceneComponent.K2_GetComponentToWorld` (`self.Arrow`)) "AdjustIfPossibleButDontSpawnIfColliding" "MultiplyWithRoot" self self)
    (set `self.bIsOneTwo` false)
    (else
      (`|SpawnActorFromClass` "/Game/Blueprint/BP_Rocket.BP_Rocket_C" (`SceneComponent.K2_GetComponentToWorld` (`self.Arrow1`)) "AdjustIfPossibleButDontSpawnIfColliding" "MultiplyWithRoot" self self)
      (set `self.bIsOneTwo` true))))

(fn `UserConstructionScript`)