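; Game mode blueprint that handles level completion once all targets are gone.
; The GameOver event counts remaining BP_Target actors and, when none are left, increments MapLevel, prints a completion message and opens Map2 after a short delay.
; The destination is hardcoded: a Format Text node that would build the map name from MapLevel is left unconnected.
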(event `GameOver`
  (bind _outactors (`GameplayStatics.GetAllActorsOfClass` "/Game/Blueprint/BP_Target.BP_Target_C"))
  (if (<= (`KismetArrayLibrary.Array_Length` _outactors) 0)
    (bind _result (`/Engine/EditorBlueprintResources/StandardMacros.IncrementInt` (`self.MapLevel`))
      (:`  `
        (set `self.MapLevel` _result)
        (`KismetSystemLibrary.PrintString` "Game Complete")
        (`KismetSystemLibrary.Delay` 2.0)
        (`GameplayStatics.OpenLevel` "Map2")))))

(fn `UserConstructionScript`)